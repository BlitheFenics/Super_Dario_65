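; Wall jump actor that pushes BP_Dario away from a wall when it overlaps one of four box triggers.
; Each overlap traces from Dario to a box for a hit normal and raises JumpMaxCount by one.
; If CanJump passes, it adds velocity along that normal, then resets the jump count after a short delay.
; Box2 and Box3 trace against Box instead of themselves, and all handlers print debug strings.
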(event OnComponentBeginOverlap(Box)
  (params (OverlappedComponent :type Primitive%20Component%20Object%20Reference) (OtherActor :type Actor%20Object%20Reference) (OtherComp :type Primitive%20Component%20Object%20Reference) (OtherBodyIndex :type Integer) (bFromSweep :type Boolean) (SweepResult :type Hit%20Result%20Structure%20%28by%20ref%29))
  (bind _asbp_dario (Utilities|Casting|CastToBP_Dario OtherActor))
  (bind _hitnormal (Collision|LineTraceComponent (Variables|Default|GetBox) (Transformation|GetActorLocation _asbp_dario) (Transformation|GetWorldLocation (Variables|Default|GetBox)) true false false))
  (Development|PrintString "Box")
  (Variables|/Script/Engine.Character|SetJumpMaxCount _asbp_dario (+ (Variables|/Script/Engine.Character|GetJumpMaxCount _asbp_dario) 1))
  (if (Character|CanJump _asbp_dario)
    (Variables|/Script/Engine.MovementComponent|SetVelocity (Pawn|GetMovementComponent _asbp_dario) (+ (* _hitnormal 1e+03) (Variables|/Script/Engine.MovementComponent|GetVelocity (Pawn|GetMovementComponent _asbp_dario))))
    (Utilities|FlowControl|Delay 0.2)
    (Variables|/Script/Engine.Character|SetJumpMaxCount _asbp_dario 1)))

(event OnComponentBeginOverlap(Box1)
  (params (OverlappedComponent :type Primitive%20Component%20Object%20Reference) (OtherActor :type Actor%20Object%20Reference) (OtherComp :type Primitive%20Component%20Object%20Reference) (OtherBodyIndex :type Integer) (bFromSweep :type Boolean) (SweepResult :type Hit%20Result%20Structure%20%28by%20ref%29))
  (bind _asbp_dario (Utilities|Casting|CastToBP_Dario OtherActor))
  (bind _hitnormal (Collision|LineTraceComponent (Variables|Default|GetBox1) (Transformation|GetActorLocation _asbp_dario) (Transformation|GetWorldLocation (Variables|Default|GetBox1)) true false false))
  (Development|PrintString "Box3")
  (Variables|/Script/Engine.Character|SetJumpMaxCount _asbp_dario (+ (Variables|/Script/Engine.Character|GetJumpMaxCount _asbp_dario) 1))
  (if (Character|CanJump _asbp_dario)
    (Variables|/Script/Engine.MovementComponent|SetVelocity (Pawn|GetMovementComponent _asbp_dario) (+ (* _hitnormal 1e+03) (Variables|/Script/Engine.MovementComponent|GetVelocity (Pawn|GetMovementComponent _asbp_dario))))
    (Utilities|FlowControl|Delay 0.2)
    (Variables|/Script/Engine.Character|SetJumpMaxCount _asbp_dario 1)))

(event OnComponentBeginOverlap(Box2)
  (params (OverlappedComponent :type Primitive%20Component%20Object%20Reference) (OtherActor :type Actor%20Object%20Reference) (OtherComp :type Primitive%20Component%20Object%20Reference) (OtherBodyIndex :type Integer) (bFromSweep :type Boolean) (SweepResult :type Hit%20Result%20Structure%20%28by%20ref%29))
  (bind _asbp_dario (Utilities|Casting|CastToBP_Dario OtherActor))
  (bind _hitnormal (Collision|LineTraceComponent (Variables|Default|GetBox) (Transformation|GetActorLocation _asbp_dario) (Transformation|GetWorldLocation (Variables|Default|GetBox)) true false false))
  (Development|PrintString "Box2")
  (Variables|/Script/Engine.Character|SetJumpMaxCount _asbp_dario (+ (Variables|/Script/Engine.Character|GetJumpMaxCount _asbp_dario) 1))
  (if (Character|CanJump _asbp_dario)
    (Variables|/Script/Engine.MovementComponent|SetVelocity (Pawn|GetMovementComponent _asbp_dario) (+ (* _hitnormal 1e+03) (Variables|/Script/Engine.MovementComponent|GetVelocity (Pawn|GetMovementComponent _asbp_dario))))
    (Utilities|FlowControl|Delay 0.2)
    (Variables|/Script/Engine.Character|SetJumpMaxCount _asbp_dario 1)))

(event OnComponentBeginOverlap(Box3)
  (params (OverlappedComponent :type Primitive%20Component%20Object%20Reference) (OtherActor :type Actor%20Object%20Reference) (OtherComp :type Primitive%20Component%20Object%20Reference) (OtherBodyIndex :type Integer) (bFromSweep :type Boolean) (SweepResult :type Hit%20Result%20Structure%20%28by%20ref%29))
  (bind _asbp_dario (Utilities|Casting|CastToBP_Dario OtherActor))
  (bind _hitnormal (Collision|LineTraceComponent (Variables|Default|GetBox) (Transformation|GetActorLocation _asbp_dario) (Transformation|GetWorldLocation (Variables|Default|GetBox)) true false false))
  (Development|PrintString "Box3")
  (Variables|/Script/Engine.Character|SetJumpMaxCount _asbp_dario (+ (Variables|/Script/Engine.Character|GetJumpMaxCount _asbp_dario) 1))
  (if (Character|CanJump _asbp_dario)
    (Variables|/Script/Engine.MovementComponent|SetVelocity (Pawn|GetMovementComponent _asbp_dario) (+ (* _hitnormal 1e+03) (Variables|/Script/Engine.MovementComponent|GetVelocity (Pawn|GetMovementComponent _asbp_dario))))
    (Utilities|FlowControl|Delay 0.2)
    (Variables|/Script/Engine.Character|SetJumpMaxCount _asbp_dario 1)))

(fn ConstructionScript)