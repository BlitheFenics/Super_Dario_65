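; Homing missile actor that strikes from above at the position of the BP_Dario player.
; On BeginPlay it launches upward, then after a short delay teleports over the player and traces down to place a target marker effect.
; A timeline lerps the flipped mesh to that fixed point, without further tracking.
; On impact it spawns a flash, removes the marker, damages the player if within range, and destroys itself.
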(event EventBeginPlay
  (bind _returnvalue (Game|GetPlayerCharacter 0))
  (bind _returnvalue_2 (Game|GetPlayerCharacter 0))
  (bind _missilemesh (Variables|Default|GetMissileMesh))
  (bind _missilemesh_2 (Variables|Default|GetMissileMesh))
  (bind _returnvalue_3 (Transformation|GetWorldLocation _missilemesh_2))
  (bind _returnvalue_4 (Transformation|GetWorldLocation _missilemesh))
  (bind _asbp_dario (Utilities|Casting|CastToBP_Dario _returnvalue))
  (bind _asbp_dario_2 (Utilities|Casting|CastToBP_Dario _returnvalue_2))
  (bind _capsulecomponent (Variables|/Script/Engine.Character|GetCapsuleComponent _asbp_dario))
  (bind _capsulecomponent_2 (Variables|/Script/Engine.Character|GetCapsuleComponent _asbp_dario_2))
  (bind _returnvalue_5 (Transformation|GetWorldLocation _capsulecomponent_2))
  (bind _returnvalue_6 (Transformation|GetWorldLocation _capsulecomponent))
  (bind _returnvalue_7 (Math|Vector|Distance(Vector) _returnvalue_6 _returnvalue_4))
  (Physics|SetPhysicsLinearVelocity (Variables|Default|GetMissileMesh) "0,0.000000,1000.000000" false "None")
  (Utilities|FlowControl|Delay 1.0)
  (Transformation|SetWorldLocation (Variables|Default|GetMissileMesh) (Math|Vector|MakeVector (.x _returnvalue_5) (.y _returnvalue_5) (.z (Transformation|GetWorldLocation (Variables|Default|GetMissileMesh)))) false true)
  (bind _outhit (Collision|LineTraceByChannel (Math|Vector|MakeVector (.x _returnvalue_3) (.y _returnvalue_3) (.z _returnvalue_3)) (Math|Vector|MakeVector (.x _returnvalue_3) (.y _returnvalue_3) -1e+03) "TraceTypeQuery1" false 0 "None"))
  (bind _output_get (Variables|Default|SettargetPoint (+ "0, 0,2.000000" (.impactpoint _outhit))))
  (bind _returnvalue_8 (Niagara|SpawnSystematLocation "/Game/VFX/TargetSystem.TargetSystem" _output_get))
  (Variables|Default|Settarget _returnvalue_8)
  (Transformation|SetWorldRotation (Variables|Default|GetMissileMesh) "0, 0,180.000000" false false)
  (Variables|Default|SetstartPoint (Transformation|GetWorldLocation (Variables|Default|GetMissileMesh)))
  (bind _newtrack_0 (Timeline|Timeline_0 PlayFromStart)
    (:Update
      (Transformation|SetWorldLocation (Variables|Default|GetMissileMesh) (Math|Vector|Lerp(Vector) (Variables|Default|GetstartPoint) (Variables|Default|GettargetPoint) _newtrack_0) false false))
    (:Finished
      (Niagara|SpawnSystematLocation "/Game/VFX/FlashSystem.FlashSystem" (Variables|Default|GettargetPoint))
      (Components|DestroyComponent (Variables|Default|Gettarget))
      (if (< _returnvalue_7 3e+02)
        (Game|Damage|ApplyDamage _asbp_dario 1.0 0 0)
        (Development|PrintString (Utilities|String|ToString(Float) _returnvalue_7)))
      (Actor|DestroyActor))))

(fn ConstructionScript)