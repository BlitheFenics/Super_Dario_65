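; Octo squid enemy that Dario can kill by jumping on its head and that hurts him with a spinning melee attack.
; A falling Dario overlapping HeadCollision bounces back, increments the game instance kill count, and triggers sound and splat effects before the enemy is destroyed.
; MeleeAttack plays the spin montage, while StartAttack and EndAttack gate damage from the Box overlap.
; Any damage received destroys the enemy outright.
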(event OnComponentBeginOverlap(Box)
  (params (OverlappedComponent :type Primitive%20Component%20Object%20Reference) (OtherActor :type Actor%20Object%20Reference) (OtherComp :type Primitive%20Component%20Object%20Reference) (OtherBodyIndex :type Integer) (bFromSweep :type Boolean) (SweepResult :type Hit%20Result%20Structure%20%28by%20ref%29))
  (bind _asbp_dario (Utilities|Casting|CastToBP_Dario OtherActor))
  (if (Variables|Default|GetIsAttacking)
    (Game|Damage|ApplyDamage _asbp_dario 1.0 0 0)))

(event OnComponentBeginOverlap(HeadCollision)
  (params (OverlappedComponent :type Primitive%20Component%20Object%20Reference) (OtherActor :type Actor%20Object%20Reference) (OtherComp :type Primitive%20Component%20Object%20Reference) (OtherBodyIndex :type Integer) (bFromSweep :type Boolean) (SweepResult :type Hit%20Result%20Structure%20%28by%20ref%29))
  (bind _returnvalue (Transformation|GetActorLocation))
  (bind _asbp_dario (Utilities|Casting|CastToBP_Dario (Game|GetPlayerCharacter 0)))
  (if (and (== (Utilities|GetClass OtherActor) "/Game/Blueprints/BP_Dario.BP_Dario_C") (< (.z (Transformation|GetVelocity _asbp_dario)) 0.0))
    (Default|BounceBack _asbp_dario)
    (bind _asdario_game_instance (Utilities|Casting|CastToDarioGameInstance (Game|GetGameInstance)))
    (Variables|/Game/DarioGameInstance.DarioGameInstance_C|SetOctoSquidsKilled _asdario_game_instance (+ (Variables|/Game/DarioGameInstance.DarioGameInstance_C|GetOctoSquidsKilled _asdario_game_instance) 1))
    (Audio|PlaySoundatLocation "/Game/Music/SoundFX/EnemyHurt_Cue.EnemyHurt_Cue" _returnvalue "0, 0, 0" 1.0 1.0 0.0 0 0 0)
    (Niagara|SpawnSystematLocation "/Game/VFX/OctoSplatSystem.OctoSplatSystem" (- _returnvalue "0,0.000000,5.000000"))
    (Actor|DestroyActor)))

(event Custom|EndAttack
  (Variables|Default|SetIsAttacking false))

(event Custom|StartAttack
  (Variables|Default|SetIsAttacking true))

(event EventBeginPlay)

(event Collision|EventActorBeginOverlap
  (params (OtherActor :type Actor%20Object%20Reference)))

(event Game|Damage|EventAnyDamage
  (params (Damage :type Float%20%28single-precision%29) (DamageType :type Damage%20Type%20Object%20Reference) (InstigatedBy :type Controller%20Object%20Reference) (DamageCauser :type Actor%20Object%20Reference))
  (Actor|DestroyActor))

(event EventMeleeAttack
  (Animation|Montage|PlayMontage (Variables|Character|GetMesh) "/Game/EnemyAssets/Trioptoquadropus/Animations/octo_spin_Montage.octo_spin_Montage" 0.5))

(fn ConstructionScript)