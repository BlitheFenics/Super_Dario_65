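; Eyeball enemy Blueprint that fires projectiles and can be killed by damage.
; Despite its name, the MeleeAttack event is a ranged attack, spawning an EyeProjectile at the ArrowDirection component's world transform.
; Any damage removes one Health regardless of amount and plays a hurt sound at the world origin rather than at the enemy.
; The actor destroys itself once Health reaches zero or below.
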(event EventBeginPlay)

(event Collision|EventActorBeginOverlap
  (params (OtherActor :type Actor%20Object%20Reference)))

(event EventTick
  (params (DeltaSeconds :type Float%20%28single-precision%29)))

(event Game|Damage|EventAnyDamage
  (params (Damage :type Float%20%28single-precision%29) (DamageType :type Damage%20Type%20Object%20Reference) (InstigatedBy :type Controller%20Object%20Reference) (DamageCauser :type Actor%20Object%20Reference))
  (Variables|Default|SetHealth (- (Variables|Default|GetHealth) 1))
  (Audio|PlaySoundatLocation "/Game/Music/SoundFX/EnemyHurt_Cue.EnemyHurt_Cue" "0, 0, 0" "0, 0, 0" 1.0 1.0 0.0 0 0 0)
  (if (<= (Variables|Default|GetHealth) 0)
    (Actor|DestroyActor)))

(event EventMeleeAttack
  (Game|SpawnActorfromClass "/Game/CarSystems/EyeProjectile.EyeProjectile_C" (Transformation|GetWorldTransform (Variables|Default|GetArrowDirection)) "Undefined" 0 0))

(fn ConstructionScript)