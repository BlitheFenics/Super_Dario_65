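; Door actor that stays blocked until the player (BP_Dario) carries enough rods.
; Entering the box trigger shows a RodsForDoorUI widget with the required count, removed on exit or success.
; With enough rods, it opens the Iris through Door_AnimBP, disables the blocker's collision, turns the light green and records DoorOpen in DarioGameInstance.
; An older timeline that raises the door is left unconnected.
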(event OnComponentBeginOverlap(Box)
  (params (OverlappedComponent :type Primitive%20Component%20Object%20Reference) (OtherActor :type Actor%20Object%20Reference) (OtherComp :type Primitive%20Component%20Object%20Reference) (OtherBodyIndex :type Integer) (bFromSweep :type Boolean) (SweepResult :type Hit%20Result%20Structure%20%28by%20ref%29))
  (bind _doorui (Variables|Default|GetDoorUI))
  (bind _rodsneeded (Variables|Default|GetRodsNeeded))
  (bind _asbp_dario (Utilities|Casting|CastToBP_Dario OtherActor))
  (UserInterface|Viewport|AddtoViewport _doorui 0)
  (Variables|/Game/Blueprints/UIBlueprints/RodsForDoorUI.RodsForDoorUI_C|SetNumRods _doorui _rodsneeded)
  (if (>= (Variables|/Script/Super_Dario_65.DarioBase|GetRods _asbp_dario) _rodsneeded)
    (Widget|RemovefromParent (Variables|Default|GetDoorUI))
    (Variables|/Game/Assets/Door/Door_AnimBP.Door_AnimBP_C|SetisOpen (.AsDoor%20Anim%20BP (Utilities|Casting|CastToDoor_AnimBP (Components|SkeletalMesh|GetAnimInstance (Variables|Default|GetIris)))) true)
    (Collision|SetCollisionEnabled (Variables|Default|GetBlocker) "NoCollision")
    (Transformation|SetRelativeLocation (Variables|Default|GetPointLight) "60.000000,67.000000,260.000000" false false)
    (Rendering|Components|Light|SetLightColor (Variables|Default|GetPointLight) "(R=0.176409,G=1.000000,B=0.000000,A=1.000000)" true)
    (bind _asdario_game_instance (Utilities|Casting|CastToDarioGameInstance (Game|GetGameInstance)))
    (Variables|/Game/DarioGameInstance.DarioGameInstance_C|SetDoorOpen _asdario_game_instance true)))

(event OnComponentEndOverlap(Box)
  (params (OverlappedComponent :type Primitive%20Component%20Object%20Reference) (OtherActor :type Actor%20Object%20Reference) (OtherComp :type Primitive%20Component%20Object%20Reference) (OtherBodyIndex :type Integer))
  (Utilities|Casting|CastToBP_Dario OtherActor)
  (Widget|RemovefromParent (Variables|Default|GetDoorUI)))

(event EventBeginPlay
  (bind _returnvalue (UserInterface|CreateWidget "/Game/Blueprints/UIBlueprints/RodsForDoorUI.RodsForDoorUI_C"))
  (Variables|Default|SetDoorUI _returnvalue))

(event Collision|EventActorBeginOverlap
  (params (OtherActor :type Actor%20Object%20Reference)))

(event EventTick
  (params (DeltaSeconds :type Float%20%28single-precision%29)))

(fn ConstructionScript)