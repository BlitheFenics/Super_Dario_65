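; BP_LightningBolt is a cinematic lightning actor that repeatedly flashes a bolt with thunder.
; On BeginPlay it waits a fixed lead-in plus a configurable Delay, strikes, then starts a looping timer whose interval is randomized once between MinFrequency and MaxFrequency.
; Each strike plays a random thunder cue at the actor, activates Niagara and briefly shows the static mesh before hiding it.
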(event Custom|CustomEvent_0
  (bind _returnvalue (Transformation|GetActorLocation))
  (switch int (Math|Random|RandomIntegerinRange 0 2)
    (:Default
      (Audio|PlaySoundatLocation "/Game/Music/SoundFX/CutsceneSFX/Thunder1_Cue.Thunder1_Cue" _returnvalue "0, 0, 0" 1.0 1.0 0.0 0 0 0 :!label _label))
    (:0
      (goto _label))
    (:1
      (Audio|PlaySoundatLocation "/Game/Music/SoundFX/CutsceneSFX/Thunder3_Cue.Thunder3_Cue" _returnvalue "0, 0, 0" 1.0 1.0 0.0 0 0 0))
    (:2
      (Audio|PlaySoundatLocation "/Game/Music/SoundFX/CutsceneSFX/Thunder4_Cue.Thunder4_Cue" _returnvalue "0, 0, 0" 1.0 1.0 0.0 0 0 0)))
  (Rendering|SetVisibility (Variables|Default|GetStaticMesh) true false)
  (Components|Activation|Activate (Variables|Default|GetNiagara) false)
  (Utilities|FlowControl|Delay 0.2)
  (Rendering|SetVisibility (Variables|Default|GetStaticMesh) false false))

(event EventBeginPlay
  (Utilities|FlowControl|Delay 24.0)
  (Utilities|FlowControl|Delay (Variables|Default|GetDelay))
  (CallFunction|CustomEvent0)
  (Utilities|Time|SetTimerbyEvent (delegate Custom|CustomEvent_0) (Math|Random|RandomFloatinRange (Variables|Default|GetMinFrequency) (Variables|Default|GetMaxFrequency)) true))

(event Collision|EventActorBeginOverlap
  (params (OtherActor :type Actor%20Object%20Reference)))

(event EventTick
  (params (DeltaSeconds :type Float%20%28single-precision%29)))

(fn ConstructionScript)