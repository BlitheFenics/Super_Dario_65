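; BP_Cloud is a cinematic cloud actor that drifts along world X and flickers with lightning.
; On BeginPlay it randomizes its rotation and starts LightningFlash, a self-repeating loop that waits a short random delay, then drives PointLight intensity from a timeline.
; Tick moves the actor by Speed scaled by delta time, and JumpAhead sets a new fixed Speed after a delay from BeginPlay.
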(event Custom|lightning%20flash
  (Utilities|FlowControl|Delay (Math|Random|RandomFloatinRange 0.1 3.0))
  (bind _newtrack_0 (Timeline|Timeline_0 PlayFromStart)
    (:Update
      (Rendering|Components|Light|SetIntensity (Variables|Default|GetPointLight) _newtrack_0))
    (:Finished
      (CallFunction|LightningFlash))))

(event Custom|jumpAhead
  (Variables|Default|SetSpeed 9e+02))

(event EventBeginPlay
  (Transformation|SetActorRotation (Math|Rotator|MakeRotator 0.0 (Math|Random|RandomFloatinRange -1.8e+02 1.8e+02) 0.0))
  (Transformation|SetActorRotation (Math|Rotator|MakeRotator 0.0 0.0 (Math|Random|RandomFloatinRange -1.8e+02 1.8e+02)))
  (CallFunction|LightningFlash)
  (Utilities|FlowControl|Delay 12.0)
  (CallFunction|JumpAhead))

(event Collision|EventActorBeginOverlap
  (params (OtherActor :type Actor%20Object%20Reference)))

(event EventTick
  (params (DeltaSeconds :type Float%20%28single-precision%29))
  (Transformation|AddActorWorldOffset (Math|Vector|MakeVector (* DeltaSeconds (Variables|Default|GetSpeed)) 0.0 0.0)))

(fn ConstructionScript)