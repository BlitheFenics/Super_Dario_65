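; Cinematic reactor cable actor, built on a cable component that can be broken loose or hidden on demand.
; Detach plays a 2D spark sound, spawns a non-auto-destroying spark burst at the cable's rotated end location, then frees that end.
; Hide turns off the cable component's visibility; nothing in the graph calls either event, and a delayed Detach is left unwired.
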(event Custom|Detach
  (Audio|PlaySound2D "/Game/Music/SoundFX/CutsceneSFX/Sparks1_Cue.Sparks1_Cue" 1.0 1.0 0.0 0 0)
  (Niagara|SpawnSystematLocation "/Game/VFX/SparkBurstSystem.SparkBurstSystem" (+ (Transformation|GetWorldLocation (Variables|Default|GetCableComponent)) (Math|Vector|RotateVector (Variables|/Script/CableComponent.CableComponent|GetEndLocation (Variables|Default|GetCableComponent)) (Transformation|GetActorRotation))) "0, 0, 0" "1.000000,1.000000,1.000000" false)
  (Variables|/Script/CableComponent.CableComponent|SetbAttachEnd (Variables|Default|GetCableComponent) false))

(event Custom|Hide
  (Rendering|SetVisibility (Variables|Default|GetCableComponent) false false))

(event EventBeginPlay)

(event Collision|EventActorBeginOverlap
  (params (OtherActor :type Actor%20Object%20Reference)))

(event EventTick
  (params (DeltaSeconds :type Float%20%28single-precision%29)))

(fn ConstructionScript)