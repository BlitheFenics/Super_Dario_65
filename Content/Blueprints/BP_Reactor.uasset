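; Reactor boss character that shows a health bar, plays a wake montage, then alternates wandering to random navigable points with volleys of homing missiles.
; BP_Dario overlapping its Head stuns it, halting movement and opening a timed vulnerability window before it recovers.
; Projectiles hitting the capsule are destroyed and only damage it while vulnerable; death flags EndGame on the game instance and opens Exterior.
; Montages and SetAnimState drive the animation Blueprint.
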(event OnComponentBeginOverlap(Head)
  (params (OverlappedComponent :type Primitive%20Component%20Object%20Reference) (OtherActor :type Actor%20Object%20Reference) (OtherComp :type Primitive%20Component%20Object%20Reference) (OtherBodyIndex :type Integer) (bFromSweep :type Boolean) (SweepResult :type Hit%20Result%20Structure%20%28by%20ref%29))
  (bind _charactermovement (Variables|Character|GetCharacterMovement))
  (Utilities|Casting|CastToBP_Dario OtherActor)
  (Variables|Default|SetStunned true)
  (Components|Movement|StopMovementImmediately _charactermovement)
  (Pawn|Components|CharacterMovement|DisableMovement _charactermovement)
  (Utilities|FlowControl|Sequence
    (:then_0
      (Utilities|FlowControl|ForLoopwithBreak 0 4) ; enters at Break
    )
    (:then_1
      (Animation|Montage|PlayMontage (Variables|Character|GetMesh) "/Game/EnemyAssets/Reactor/Animations/Reactor_Stun_Montage.Reactor_Stun_Montage"
        (:then
          (CallFunction|SetAnimState 2))
        (:OnCompleted
          (Variables|Default|Setvulnerable true)
          (Utilities|FlowControl|Delay 8.0)
          (Animation|Montage|PlayMontage (Variables|Character|GetMesh) "/Game/EnemyAssets/Reactor/Animations/Reactor_Recover_Montage.Reactor_Recover_Montage"
            (:then
              (CallFunction|SetAnimState 1)
              (Variables|Default|SetStunned false)
              (Variables|Default|Setvulnerable false))
            (:OnCompleted
              (Pawn|Components|CharacterMovement|SetMovementMode (Variables|Character|GetCharacterMovement) "MOVE_Walking" 0)
              (CallFunction|BeginWander))))))))

(event OnComponentBeginOverlap(CapsuleComponent)
  (params (OverlappedComponent :type Primitive%20Component%20Object%20Reference) (OtherActor :type Actor%20Object%20Reference) (OtherComp :type Primitive%20Component%20Object%20Reference) (OtherBodyIndex :type Integer) (bFromSweep :type Boolean) (SweepResult :type Hit%20Result%20Structure%20%28by%20ref%29))
  (bind _asprojectile (Utilities|Casting|CastToProjectile OtherActor))
  (Actor|DestroyActor _asprojectile)
  (if (Variables|Default|Getvulnerable)
    (Math|Integer|DecrementInt (Variables|Default|Gethealth)
      (:%20%20
        (Variables|/Game/UI/BossHealthBar.BossHealthBar_C|Sethealth (Variables|Default|GetheathBar) (Variables|Default|Gethealth))
        (if (<= (Variables|Default|Gethealth) 0)
          (CallFunction|Death))))))

(event Custom|BeginWander
  (CallFunction|SetAnimState 1)
  (AI|AIMoveTo self (.RandomLocation (Class|NavigationSystemV1|GetRandomPointinNavigableRadius (Transformation|GetActorLocation) (Variables|Default|GetWander%20Radius) 0 0)) 0 5.0 true
    (:OnSuccess
      _)
    (:OnFail
      _))
  (if (not (Variables|Default|GetStunned))
    (CallFunction|SetAnimState)
    (Utilities|FlowControl|ForLoopwithBreak 0 4
      (:LoopBody
        (Utilities|FlowControl|Delay 0.8)
        (Game|SpawnActorfromClass "/Game/Blueprints/HomingMissileBP.HomingMissileBP_C" (Math|Transform|MakeTransform (Transformation|GetWorldLocation (Variables|Default|GetArrow1)) "0, 0, 0" "1,1,1") "Undefined" 0 0))
      (:Completed
        (if (not (Variables|Default|GetStunned))
          (CallFunction|BeginWander))))))

(event Custom|Death
  (bind _returnvalue (Game|GetGameInstance))
  (bind _asdario_game_instance (Utilities|Casting|CastToDarioGameInstance _returnvalue))
  (Widget|RemovefromParent (Variables|Default|GetheathBar))
  (Variables|/Game/DarioGameInstance.DarioGameInstance_C|SetEndGame _asdario_game_instance true)
  (Variables|/Script/Super_Dario_65.Dario64GameInstance|SetcurrentLevel _asdario_game_instance 10)
  (Game|OpenLevel(byName) "Exterior"))

(event EventBeginPlay
  (bind _returnvalue (UserInterface|CreateWidget "/Game/UI/BossHealthBar.BossHealthBar_C"))
  (bind _output_get (Variables|Default|SetheathBar _returnvalue))
  (Variables|/Game/UI/BossHealthBar.BossHealthBar_C|Sethealth _output_get (Variables|Default|Gethealth))
  (Variables|/Game/UI/BossHealthBar.BossHealthBar_C|SetmaxHealth _output_get (Variables|Default|Gethealth))
  (UserInterface|Viewport|AddtoViewport _output_get 0)
  (CallFunction|SetAnimState 3)
  (Utilities|FlowControl|Delay 3.0)
  (Animation|Montage|PlayMontage (Variables|Character|GetMesh) "/Game/EnemyAssets/Reactor/Animations/Reactor_wake_Montage.Reactor_wake_Montage"
    (:then
      (CallFunction|SetAnimState 1))
    (:OnCompleted
      (CallFunction|BeginWander))))

(event Collision|EventActorBeginOverlap
  (params (OtherActor :type Actor%20Object%20Reference)))

(event EventTick
  (params (DeltaSeconds :type Float%20%28single-precision%29)))

(fn ConstructionScript)

(fn SetAnimState
  (params (NewParam :type Integer))
  (bind _asreactor_anim_bp (Utilities|Casting|CastToReactor_AnimBP (Components|SkeletalMesh|GetAnimInstance (Variables|Character|GetMesh))))
  (Variables|/Game/EnemyAssets/Reactor/Animations/Reactor_AnimBP.Reactor_AnimBP_C|SetAnimState _asreactor_anim_bp NewParam))