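; BeerPickup is a collectible beer mug actor that the BP_Dario player gathers by touching it.
; On actor overlap it increments Dario's MugshotCollected and the DarioGameInstance's TotalMugsCollected.
; It then prints the total, plays a collect sound at the world origin rather than its own position, and destroys itself.
; The box collider's own overlap event is empty.
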(event OnComponentBeginOverlap(BoxColider)
  (params (OverlappedComponent :type Primitive%20Component%20Object%20Reference) (OtherActor :type Actor%20Object%20Reference) (OtherComp :type Primitive%20Component%20Object%20Reference) (OtherBodyIndex :type Integer) (bFromSweep :type Boolean) (SweepResult :type Hit%20Result%20Structure%20%28by%20ref%29)))

(event EventBeginPlay)

(event EventTick
  (params (DeltaSeconds :type Float%20%28single-precision%29)))

(event Collision|EventActorBeginOverlap
  (params (OtherActor :type Actor%20Object%20Reference))
  (bind _asbp_dario (Utilities|Casting|CastToBP_Dario OtherActor))
  (Variables|/Script/Super_Dario_65.DarioBase|SetMugshotCollected _asbp_dario (+ (Variables|/Script/Super_Dario_65.DarioBase|GetMugshotCollected _asbp_dario) 1))
  (bind _asdario_game_instance (Utilities|Casting|CastToDarioGameInstance (Game|GetGameInstance)))
  (bind _output_get (Variables|/Script/Super_Dario_65.Dario64GameInstance|SettotalMugsCollected _asdario_game_instance (+ (Variables|/Script/Super_Dario_65.Dario64GameInstance|GettotalMugsCollected _asdario_game_instance) 1)))
  (Development|PrintString (Utilities|String|ToString(Integer) _output_get))
  (Audio|PlaySoundatLocation "/Game/Music/SoundFX/CollectSound_Cue.CollectSound_Cue" "0, 0, 0" "0, 0, 0" 1.0 1.0 0.0 0 0 0)
  (Actor|DestroyActor))

(fn ConstructionScript)