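; Computer terminal that sends Dario to its DestinationLevel via the loading level.
; Its box overlap shows a prompt, with level stats for destinations 2 and 3, and registers it as Dario's target; destination 3 requires a completed Level One time.
; TheParticleEvent plays effects, counts the use, saves the current level's stats and the new destination to the game instance, then opens LoadingLevel after a delay.
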(event OnComponentBeginOverlap(Box)
  (params (OverlappedComponent :type Primitive%20Component%20Object%20Reference) (OtherActor :type Actor%20Object%20Reference) (OtherComp :type Primitive%20Component%20Object%20Reference) (OtherBodyIndex :type Integer) (bFromSweep :type Boolean) (SweepResult :type Hit%20Result%20Structure%20%28by%20ref%29))
  (bind _a_prompt (Variables|Default|Geta_Prompt))
  (bind _destinationlevel (Variables|Default|GetDestinationLevel))
  ;[1 1 1] Showing Level stats
  (bind _asbp_dario (Utilities|Casting|CastToBP_Dario OtherActor))
  (UserInterface|Viewport|AddtoViewport _a_prompt 0)
  (if (== _destinationlevel 2)
    (Widget|SetVisibility (Variables|/Game/Blueprints/UIBlueprints/A_Prompt.A_Prompt_C|GetLevelStatsUI _a_prompt) "Visible")
    (Variables|Default|SetinRange true :!label _label)
    (Class|DarioBase|SetTargetComputer _asbp_dario self)
    (elif (== _destinationlevel 3)
      (Widget|SetVisibility (Variables|/Game/Blueprints/UIBlueprints/A_Prompt.A_Prompt_C|GetLevelStatsUI_2 _a_prompt) "Visible")
      (if (> (.timecompleted (Variables|/Script/Super_Dario_65.Dario64GameInstance|GetlevelOne (.AsDario%20Game%20Instance (Utilities|Casting|CastToDarioGameInstance (Game|GetGameInstance))))) 0.0)
        (goto _label))
      (else
        (goto _label)))))

(event OnComponentEndOverlap(Box)
  (params (OverlappedComponent :type Primitive%20Component%20Object%20Reference) (OtherActor :type Actor%20Object%20Reference) (OtherComp :type Primitive%20Component%20Object%20Reference) (OtherBodyIndex :type Integer))
  (bind _asbp_dario (Utilities|Casting|CastToBP_Dario OtherActor))
  (Widget|RemovefromParent (Variables|Default|Geta_Prompt))
  (Variables|Default|SetinRange false)
  (Class|DarioBase|ClearTargetComputer _asbp_dario))

(event EventBeginPlay
  (bind _returnvalue (UserInterface|CreateWidget "/Game/Blueprints/UIBlueprints/A_Prompt.A_Prompt_C"))
  (Variables|Default|Seta_Prompt _returnvalue)
  (Variables|Default|SetDarioPosition (Transformation|GetWorldLocation (Variables|Default|GetNiagara))))

(event Collision|EventActorBeginOverlap
  (params (OtherActor :type Actor%20Object%20Reference)))

(event EventTick
  (params (DeltaSeconds :type Float%20%28single-precision%29)))

(event EventTheParticleEvent
  (Audio|PlaySoundatLocation "/Game/Music/SoundFX/ComputerNoise_Cue.ComputerNoise_Cue" "0, 0, 0" "0, 0, 0" 1.0 1.0 0.0 0 0 0)
  (Components|Activation|Activate (Variables|Default|GetNiagara) false)
  (bind _asdario_game_instance (Utilities|Casting|CastToDarioGameInstance (Game|GetGameInstance)))
  (Variables|/Game/DarioGameInstance.DarioGameInstance_C|SetComputersUsed _asdario_game_instance (+ (Variables|/Game/DarioGameInstance.DarioGameInstance_C|GetComputersUsed _asdario_game_instance) 1))
  (Development|PrintString (Utilities|String|ToString(Integer) (Variables|/Game/DarioGameInstance.DarioGameInstance_C|GetComputersUsed _asdario_game_instance)))
  (Widget|RemovefromParent (Variables|Default|Geta_Prompt))
  (CallFunction|SaveLevelStats)
  (Utilities|FlowControl|Delay 9.0)
  (Game|OpenLevel(byName) "LoadingLevel"))

(fn ConstructionScript)

(fn SaveLevelStats
  (bind _returnvalue (Game|GetGameInstance))
  (bind _asdario_game_instance (Utilities|Casting|CastToDarioGameInstance _returnvalue))
  (bind _asbp_dario (Utilities|Casting|CastToBP_Dario (Game|Player|GetPlayerPawn 0)))
  (if (== (Variables|/Script/Super_Dario_65.Dario64GameInstance|GetcurrentLevel _asdario_game_instance) 2)
    (Variables|/Script/Super_Dario_65.Dario64GameInstance|SetlevelOne _asdario_game_instance (Utilities|Struct|MakeULevelStats (Variables|/Script/Super_Dario_65.DarioBase|GetRods _asbp_dario) (Variables|/Game/Blueprints/BP_Dario.BP_Dario_C|GetBeerPickedUp _asbp_dario) (Variables|/Script/Super_Dario_65.DarioBase|GetBulletsFired _asbp_dario) (Variables|/Script/Super_Dario_65.DarioBase|GetMugshotCollected _asbp_dario) (Variables|/Game/Blueprints/BP_Dario.BP_Dario_C|GetTime _asbp_dario)))
    (Default|SaveLevel1Times _asdario_game_instance (Variables|/Game/Blueprints/BP_Dario.BP_Dario_C|GetTime _asbp_dario))
    (elif (== (Variables|/Script/Super_Dario_65.Dario64GameInstance|GetcurrentLevel _asdario_game_instance) 3)
      (Variables|/Script/Super_Dario_65.Dario64GameInstance|SetlevelTwo _asdario_game_instance (Utilities|Struct|MakeULevelStats (Variables|/Script/Super_Dario_65.DarioBase|GetRods _asbp_dario) (Variables|/Game/Blueprints/BP_Dario.BP_Dario_C|GetBeerPickedUp _asbp_dario) (Variables|/Script/Super_Dario_65.DarioBase|GetBulletsFired _asbp_dario) (Variables|/Script/Super_Dario_65.DarioBase|GetMugshotCollected _asbp_dario) (Variables|/Game/Blueprints/BP_Dario.BP_Dario_C|GetTime _asbp_dario)))
      (Default|SaveLevel2Times _asdario_game_instance (Variables|/Game/Blueprints/BP_Dario.BP_Dario_C|GetTime _asbp_dario))))
  (Variables|/Script/Super_Dario_65.Dario64GameInstance|SetcurrentLevel _asdario_game_instance (Variables|Default|GetDestinationLevel))
  (Default|SaveGame _asdario_game_instance))