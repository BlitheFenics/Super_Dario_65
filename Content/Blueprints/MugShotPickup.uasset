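; MugShotPickup is a beer pickup that heals and scores for the player character, BP_Dario.
; On overlap with BP_Dario, it increments the character's beer count and adds one Health if that is below the hardcoded cap.
; Both branches then increment the collected total in DarioGameInstance, play a collect sound at the world origin rather than the pickup's position, and destroy the actor.
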(event EventBeginPlay)

(event Collision|EventActorBeginOverlap
  (params (OtherActor :type Actor%20Object%20Reference))
  (bind _asbp_dario (Utilities|Casting|CastToBP_Dario OtherActor))
  (Variables|/Game/Blueprints/BP_Dario.BP_Dario_C|SetBeerPickedUp _asbp_dario (+ (Variables|/Game/Blueprints/BP_Dario.BP_Dario_C|GetBeerPickedUp _asbp_dario) 1))
  (if (< (Variables|/Script/Super_Dario_65.DarioBase|GetHealth _asbp_dario) 5)
    (Variables|/Script/Super_Dario_65.DarioBase|SetHealth _asbp_dario (+ (Variables|/Script/Super_Dario_65.DarioBase|GetHealth _asbp_dario) 1))
    (bind _asdario_game_instance (Utilities|Casting|CastToDarioGameInstance (Game|GetGameInstance)))
    (Variables|/Script/Super_Dario_65.Dario64GameInstance|SettotalBeerCollected _asdario_game_instance (+ (Variables|/Script/Super_Dario_65.Dario64GameInstance|GettotalBeerCollected _asdario_game_instance) 1))
    (Audio|PlaySoundatLocation "/Game/Music/SoundFX/CollectSound_Cue.CollectSound_Cue" "0, 0, 0" "0, 0, 0" 1.0 1.0 0.0 0 0 0)
    (Actor|DestroyActor)
    (else
      (bind _asdario_game_instance_2 (Utilities|Casting|CastToDarioGameInstance (Game|GetGameInstance)))
      (Variables|/Script/Super_Dario_65.Dario64GameInstance|SettotalBeerCollected _asdario_game_instance_2 (+ (Variables|/Script/Super_Dario_65.Dario64GameInstance|GettotalBeerCollected _asdario_game_instance_2) 1))
      (Audio|PlaySoundatLocation "/Game/Music/SoundFX/CollectSound_Cue.CollectSound_Cue" "0, 0, 0" "0, 0, 0" 1.0 1.0 0.0 0 0 0)
      (Actor|DestroyActor))))

(event EventTick
  (params (DeltaSeconds :type Float%20%28single-precision%29)))

(fn ConstructionScript)