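; PickupsBP is a collectible rod pickup that the BP_Dario character collects by overlapping it.
; On overlap it increments the character's Rods count, then the TotalRodsCollected tally in DarioGameInstance.
; It then plays a collect sound at the world origin, spawns a flash effect at its own location and destroys itself.
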(event EventBeginPlay)

(event Collision|EventActorBeginOverlap
  (params (OtherActor :type Actor%20Object%20Reference))
  (bind _asbp_dario (Utilities|Casting|CastToBP_Dario OtherActor))
  (Variables|/Script/Super_Dario_65.DarioBase|SetRods _asbp_dario (+ (Variables|/Script/Super_Dario_65.DarioBase|GetRods _asbp_dario) 1))
  (bind _asdario_game_instance (Utilities|Casting|CastToDarioGameInstance (Game|GetGameInstance)))
  (Variables|/Script/Super_Dario_65.Dario64GameInstance|SettotalRodsCollected _asdario_game_instance (+ (Variables|/Script/Super_Dario_65.Dario64GameInstance|GettotalRodsCollected _asdario_game_instance) 1))
  (Audio|PlaySoundatLocation "/Game/Music/SoundFX/CollectSound_Cue.CollectSound_Cue" "0, 0, 0" "0, 0, 0" 1.0 1.0 0.0 0 0 0)
  (Niagara|SpawnSystematLocation "/Game/VFX/rodFlashSystem.rodFlashSystem" (Transformation|GetActorLocation))
  (Actor|DestroyActor))

(event EventTick
  (params (DeltaSeconds :type Float%20%28single-precision%29)))

(fn ConstructionScript)