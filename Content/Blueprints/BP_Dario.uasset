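; Dario player character Blueprint, handling health, attack, pause and HUD for the hub, level and boss maps.
; BeginPlay adds the HUD, enables pausing on those maps and applies a green, tuned Duigi variant from the game instance flag.
; With a gun, a button briefly enables a damage box against enemies; damage grants temporary immunity or, at zero health, loads LoseLevel.
; Pause and controller-disconnect screens freeze play through global time dilation.
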(event OnComponentBeginOverlap(Box1)
  (params (OverlappedComponent :type Primitive%20Component%20Object%20Reference) (OtherActor :type Actor%20Object%20Reference) (OtherComp :type Primitive%20Component%20Object%20Reference) (OtherBodyIndex :type Integer) (bFromSweep :type Boolean) (SweepResult :type Hit%20Result%20Structure%20%28by%20ref%29))
  (bind _asenemy_aibp_2 (Utilities|Casting|CastToEnemy_AIBP_2 OtherActor))
  (Game|Damage|ApplyDamage _asenemy_aibp_2 1.0 0 0))

(event Custom|BounceBack
  (Character|LaunchCharacter "0, 0,3000.000000" false false))

(event EventBeginPlay
  (Collision|SetCollisionEnabled (Variables|Default|GetBox1) "NoCollision")
  (Class|DarioBase|DisableGun)
  (bind _asdario_game_instance (Utilities|Casting|CastToDarioGameInstance (Game|GetGameInstance)))
  (if (Variables|/Game/DarioGameInstance.DarioGameInstance_C|GetdarioDuigi _asdario_game_instance)
    (Rendering|Material|SetMaterial (Variables|Character|GetMesh) 0 "/Game/Assets/Door/GreenGlass_mat.GreenGlass_mat")
    (Variables|Default|SetSprint 1.5)
    (Variables|Default|SetHighJumping 1.2)
    (Variables|/Script/Engine.CharacterMovementComponent|SetJumpZVelocity (Variables|Character|GetCharacterMovement) 3e+03))
  ;[1 1 1] HUD display
  (bind _returnvalue (Game|GetCurrentLevelName true))
  (if (Utilities|Enum|Equal(Enum) _returnvalue "HubWorld")
    (bind _returnvalue_2 (UserInterface|CreateWidget "/Game/Blueprints/UIBlueprints/DarioHUD.DarioHUD_C" :!label _label))
    (UserInterface|Viewport|AddtoViewport _returnvalue_2 0)
    (Variables|Default|SetInMenus true)
    (elif (Utilities|Enum|Equal(Enum) _returnvalue "Level1")
      (goto _label)
      (elif (Utilities|Enum|Equal(Enum) _returnvalue "Level2")
        (goto _label)
        (elif (Utilities|Enum|Equal(Enum) _returnvalue "Boss1")
          (goto _label))))))

(event EventTick
  (params (DeltaSeconds :type Float%20%28single-precision%29))
  (Variables|Default|SetTime (+ (Variables|Default|GetTime) DeltaSeconds)))

(event Game|Damage|EventAnyDamage
  (params (Damage :type Float%20%28single-precision%29) (DamageType :type Damage%20Type%20Object%20Reference) (InstigatedBy :type Controller%20Object%20Reference) (DamageCauser :type Actor%20Object%20Reference))
  (if (not (Variables|Default|Getimmune))
    (Variables|Default|SetHealth (- (Variables|Default|GetHealth) 1))
    (Audio|PlaySoundatLocation "/Game/Music/SoundFX/DarioHurt_Cue.DarioHurt_Cue" (Transformation|GetActorLocation) "0, 0, 0" 1.0 1.0 0.0 0 0 0)
    (if (<= (Variables|Default|GetHealth) 0)
      (Rendering|SetVisibility (Variables|Character|GetMesh) true false)
      (Pawn|Components|CharacterMovement|DisableMovement (Variables|Character|GetCharacterMovement))
      (Rendering|SetVisibility (Variables|Character|GetMesh) false false)
      (Rendering|SetVisibility (Variables|Default|GetMeshComp) false false)
      (Niagara|SpawnSystematLocation "/Game/VFX/Dario_DeathSystem.Dario_DeathSystem" (Transformation|GetActorLocation))
      (Audio|PlaySound2D "/Game/Music/SoundFX/Death_explosion.Death_explosion" 1.0 1.0 0.0 0 0)
      (Utilities|FlowControl|Delay 3.0)
      (Game|OpenLevel(byName) "LoseLevel")
      (else
        (Niagara|SpawnSystematLocation "/Game/VFX/BloodSystem.BloodSystem" (Transformation|GetActorLocation))
        (Variables|Default|Setimmune true)
        (Utilities|FlowControl|Delay 1.0)
        (Variables|Default|Setimmune false)))))

(event EventOnControllerConnectionChange
  (params (Connected :type Boolean) (UserID :type Integer) (ControllerID :type Integer))
  (Variables|Default|SetControllerConnected Connected)
  (if (== 0 ControllerID)
    (if (Variables|Default|GetControllerConnected)
      (Utilities|Time|SetGlobalTimeDilation 1.0)
      (Widget|RemovefromParent (Variables|Default|GetControllerDisconnect))
      (else
        (Utilities|Time|SetGlobalTimeDilation 0.0)
        (bind _returnvalue (UserInterface|CreateWidget "/Game/Blueprints/UIBlueprints/ControllerPullUI.ControllerPullUI_C"))
        (bind _output_get (Variables|Default|SetControllerDisconnect _returnvalue))
        (UserInterface|Viewport|AddtoViewport _output_get 0)))))

(event Input|GamepadEvents|GamepadSpecialRight
  (params (Key :type Key%20Structure :default "None"))
  ;[1 1 1] Pause Control
  (:Pressed
    (if (Variables|Default|GetInMenus)
      (if (> (Class|GameplayStatics|GetGlobalTimeDilation) 0.1)
        (Utilities|Time|SetGlobalTimeDilation 0.0)
        (bind _activeplayercontroller (CallFunction|GetActivePlayercontroller))
        (bind _returnvalue (UserInterface|CreateWidget "/Game/Blueprints/UIBlueprints/PauseUI.PauseUI_C" _activeplayercontroller))
        (bind _output_get (Variables|Default|SetPauseUI _returnvalue))
        (UserInterface|Viewport|AddtoViewport _output_get 0)
        (Input|SetInputModeGameandUI _activeplayercontroller (Variables|/Game/Blueprints/UIBlueprints/UIButton.UIButton_C|GetMyButton (Variables|/Game/Blueprints/UIBlueprints/PauseUI.PauseUI_C|GetResume _returnvalue)) "DoNotLock" true)
        (else
          (Utilities|Time|SetGlobalTimeDilation 1.0)
          (Widget|RemovefromParent (Variables|Default|GetPauseUI)))))))

(event Input|GamepadEvents|GamepadFaceButtonLeft
  (params (Key :type Key%20Structure :default "None"))
  (bind _box1 (Variables|Default|GetBox1))
  (:Pressed
    (if (Variables|Default|GethasGun)
      (Collision|SetCollisionEnabled _box1 "QueryAndPhysics")
      (Utilities|FlowControl|Delay 1.0)
      (Collision|SetCollisionEnabled _box1 "NoCollision"))))

(fn ConstructionScript)